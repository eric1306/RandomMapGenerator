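; Procedural dungeon enemy that wanders at random and chases hero-tagged actors entering its Trigger volume.
; A self-repeating CheckForPlayers loop uses AI MoveTo toward either the stored hero or a random navigable point, spawning an AI_Destination actor at each wander point.
; Trigger overlaps switch the chase flag for heroes and re-run the loop for any actor, with debug prints on entry.
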(event OnComponentBeginOverlap(Trigger)
  (params (OverlappedComponent :type Primitive%20Component%20Object%20Reference) (OtherActor :type Actor%20Object%20Reference) (OtherComp :type Primitive%20Component%20Object%20Reference) (OtherBodyIndex :type Integer) (bFromSweep :type Boolean) (SweepResult :type Hit%20Result%20Structure%20%28by%20ref%29))
  (if (Actor|ActorHasTag OtherActor (Variables|Default|GetHeroTag))
    (Variables|Default|SetOther%20Actor OtherActor)
    (Variables|Default|SetIsChasing true)
    (Development|PrintString (Utilities|GetObjectName (Variables|Default|GetOther%20Actor)) true true "(R=1.000000,G=0.000000,B=0.000000,A=1.000000)")
    (CallFunction|CheckforPlayers)
    (else
      (CallFunction|CheckforPlayers)
      (Development|PrintString (Utilities|String|ToString(Name) (stale _array_element)) true true "(R=0.056731,G=1.000000,B=0.264409,A=1.000000)"))))

(event OnComponentEndOverlap(Trigger)
  (params (OverlappedComponent :type Primitive%20Component%20Object%20Reference) (OtherActor :type Actor%20Object%20Reference) (OtherComp :type Primitive%20Component%20Object%20Reference) (OtherBodyIndex :type Integer))
  (if (Actor|ActorHasTag OtherActor (Variables|Default|GetHeroTag))
    (Variables|Default|SetIsChasing false)
    (CallFunction|CheckforPlayers)
    (else
      (CallFunction|CheckforPlayers))))

(event Custom|Check%20for%20Players
  (if (Variables|Default|GetIsChasing)
    (AI|AIMoveTo self "0, 0, 0" (Variables|Default|GetOther%20Actor) 5.0 false
      (:OnSuccess
        _)
      (:OnFail
        _))
    (CallFunction|CheckforPlayers)
    (else
      (bind _randomlocation (Class|NavigationSystemV1|GetRandomLocationinNavigableRadius (Transformation|GetActorLocation) 2e+03 0 0))
      (Game|SpawnActorfromClass "/Game/Procedural_Dungeon/Characters/AI_Destination.AI_Destination_C" (Math|Transform|MakeTransform _randomlocation "0, 0, 0" "1.000000,1.000000,1.000000") "AlwaysSpawn" "MultiplyWithRoot" 0 0)
      (AI|AIMoveTo self _randomlocation 0 5.0 false
        (:OnSuccess
          _)
        (:OnFail
          _))
      (CallFunction|CheckforPlayers))))

(event EventBeginPlay
  (CallFunction|CheckforPlayers))

(fn ConstructionScript)